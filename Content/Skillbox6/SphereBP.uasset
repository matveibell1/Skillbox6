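; SphereBP is an actor that moves in a straight line and bounces off whatever blocks it, losing speed with each bounce.
; Tick moves it by a swept world offset from Direction and Speed, scaled by delta time, and reflects Direction about the hit normal on a blocking hit.
; Each hit subtracts a fixed step, a tenth of the starting Speed cached at BeginPlay, while Speed exceeds MinSpeed.
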(event `self.ReceiveBeginPlay`
  (set `self.10 PercentSpeed` (* (`self.Speed`) 0.1)))

(event `self.ReceiveTick`
  (params (DeltaSeconds :type "Float (single-precision)"))
  (bind _sweephitresult (`self.K2_AddActorWorldOffset` (* (* (`self.Direction`) (`self.Speed`)) DeltaSeconds) true))
  (bind (_bblockinghit _binitialoverlap _time _distance _location _impactpoint _normal) (`GameplayStatics.BreakHitResult` _sweephitresult))
  (if _bblockinghit
    (set `self.Direction` (`KismetMathLibrary.GetReflectionVector` (`self.Direction`) _normal))
    (if (> (`self.Speed`) (`self.MinSpeed`))
      (set `self.Speed` (- (`self.Speed`) (`self.10 PercentSpeed`))))))

(fn `UserConstructionScript`)